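; AI controller for TUH AI characters that runs a behavior tree and starts wandering pawns on a route.
; On possess it sets up the blackboard, runs the tree and, if the character is flagged Wandering, writes that flag and the nearest RouteNode to the blackboard.
; The nearest node comes from a squared-distance scan of all RouteNode actors.
; Perception updates are forwarded to OnAIPerceptionUpdated, which is not defined in these graphs.
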(event OnPerceptionUpdated(AIPerception)
  (params (UpdatedActors :type Array%20of%20Actor%20Object%20References))
  (Class|TUHAIController|OnAIPerceptionUpdated UpdatedActors))

(event EventBeginPlay)

(event EventTick
  (params (DeltaSeconds :type Float%20%28single-precision%29)))

(event EventOnPossess
  (params (PossessedPawn :type Pawn%20Object%20Reference))
  (bind _self self)
  (bind _returnvalue (AI|GetBlackboard _self))
  (CallFunction|UseBlackboardDataAsset)
  (AI|RunBehaviorTree (Variables|Default|GetBehaviorTree))
  (bind _asbp_tuh_aicharacter (Utilities|Casting|CastToBP_TUH_AICharacter (Pawn|GetControlledPawn)))
  (if (Variables|/Game/Blueprints/AI/BP_TUH_AICharacter.BP_TUH_AICharacter_C|GetWandering _asbp_tuh_aicharacter)
    (bind _node (CallFunction|GetClosestNode))
    (AI|Components|Blackboard|SetValueasObject _returnvalue (Utilities|Name|MakeLiteralName "Route") _node)
    (AI|Components|Blackboard|SetValueasBool _returnvalue (Utilities|Name|MakeLiteralName "Wandering") true)))

(fn ConstructionScript)

(fn UseBlackboardDataAsset
  (Class|AIController|UseBlackboard "/Game/Blueprints/AI/Behaviors/AIBlackboard.AIBlackboard"))

(fn GetClosestNode
  (bind _outactors (Actor|GetAllActorsOfClass "/Game/Blueprints/AI/Routes/RouteNode.RouteNode_C"))
  (LocalVariables|SetMinDistance 99999999999.0)
  (for _array_element _outactors
    (if (< (Math|Vector|VectorLengthSquared (- (Transformation|GetActorLocation _array_element) (Transformation|GetActorLocation (Pawn|GetControlledPawn)))) (LocalVariables|GetMinDistance))
      (LocalVariables|SetClosestNode _array_element)
      (LocalVariables|SetMinDistance (Math|Vector|VectorLengthSquared (- (Transformation|GetActorLocation _array_element) (Transformation|GetActorLocation (Pawn|GetControlledPawn)))))))
  (return (LocalVariables|GetClosestNode)))