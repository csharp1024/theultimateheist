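; AI character Blueprint for The Ultimate Heist that converts sight, hearing and damage stimuli into detection amounts.
; UpdateStimuli dispatches by sense class: damage returns a flat maximum, while hearing falls off with log10 of distance.
; Sight requires line of sight and scales with target concealment, facing dot product, frame time, DetectSpeed and distance, switching to logarithmic falloff beyond CloseDistance.
; DetectedActor sets the blackboard Alerted flag and drops its own Concealment.
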(event EventDetectedActor
  (params (Actor :type Actor%20Object%20Reference))
  (bind _returnvalue (Pawn|GetController))
  (bind _returnvalue_2 (AI|GetBlackboard _returnvalue))
  (Utilities|IsValid _returnvalue_2
    (:Is%20Valid
      (AI|Components|Blackboard|SetValueasBool _returnvalue_2 (Utilities|Name|MakeLiteralName "Alerted") true)
      (Variables|Default|SetConcealment -1e+02))))

(fn ConstructionScript
  (|CallParentFunction))

(fn ProcessSight
  (params (Actor :type Actor%20Object%20Reference) (ReceiverLocation :type Vector :default "0, 0, 0") (StimulusLocation :type Vector :default "0, 0, 0"))
  (bind _returnvalue (- StimulusLocation ReceiverLocation))
  (bind _closedistance (Variables|Default|GetCloseDistance))
  (bind _returnvalue_2 (Math|Vector|VectorLength _returnvalue))
  (bind _asthe_ultimate_heist_character (Utilities|Casting|CastToTheUltimateHeistCharacter Actor))
  (return (* (- 1e+02 (Variables|/Script/TheUltimateHeist.TheUltimateHeistCharacter|GetConcealment _asthe_ultimate_heist_character)) (Math|Float|SelectFloat (/ (Math|Vector|DotProduct (Math|Vector|Normalize _returnvalue) (Transformation|GetActorForwardVector)) (Math|Float|SelectFloat (/ (Math|Float|Loge (- _returnvalue_2 _closedistance)) (Math|Float|Loge 1e+01)) (/ _returnvalue_2 (Variables|Default|GetCloseDistance)) (> _returnvalue_2 _closedistance))) 0.0 (Controller|LineOfSightTo (Pawn|GetController) Actor "0, 0, 0" true)) (Utilities|Time|GetWorldDeltaSeconds) (Variables|Default|GetDetectSpeed))))

(fn ProcessHearing
  (params (Actor :type Actor%20Object%20Reference) (ReceiverLocation :type Vector :default "0, 0, 0") (StimulusLocation :type Vector :default "0, 0, 0"))
  (return (/ 1e+02 (/ (Math|Float|Loge (Math|Vector|VectorLength (- ReceiverLocation StimulusLocation))) (Math|Float|Loge 1e+01)))))

(fn ProcessDamage
  (params (Actor :type Actor%20Object%20Reference) (ReceiverLocation :type Vector) (StimulusLocation :type Vector))
  (return 1e+02))

(fn UpdateStimuli
  (params (Actor :type Actor%20Object%20Reference) (StimulusAmount :type Float%20%28single-precision%29) (ReceiverLocation :type Vector :default "0, 0, 0") (StimulusLocation :type Vector :default "0, 0, 0") (SenseClass :type AI%20Sense%20Class%20Reference))
  (if (== SenseClass "/Script/AIModule.AISense_Sight")
    (bind _value (CallFunction|ProcessSight Actor ReceiverLocation StimulusLocation))
    (LocalVariables|SetValue _value)
    (elif (== SenseClass "/Script/AIModule.AISense_Hearing")
      (bind _value_2 (CallFunction|ProcessHearing Actor ReceiverLocation StimulusLocation))
      (LocalVariables|SetValue _value_2)
      (elif (== SenseClass "/Script/AIModule.AISense_Damage")
        (bind _value_3 (CallFunction|ProcessDamage Actor ReceiverLocation StimulusLocation))
        (LocalVariables|SetValue _value_3))))
  (return (LocalVariables|GetValue)))