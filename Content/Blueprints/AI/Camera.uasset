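; AI security camera that detects player characters by sight and flags the Alerted key on its controller's blackboard on detection.
; UpdateStimuli scales sight gain by inverse character Concealment, line of sight, frame time and DetectSpeed.
; Setters and getters expose the sensed-actor list and key/value arrays, while the construction script sets the camera's yaw from BaseDirection.
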(event EventBeginPlay)

(event EventActorBeginOverlap
  (params (OtherActor :type Actor%20Object%20Reference)))

(event EventTick
  (params (DeltaSeconds :type Float%20%28single-precision%29)))

(event EventSetActivelySensedActors
  (params (Actors :type Array%20of%20Actor%20Object%20References))
  (Variables|Default|SetActivelySensedActors Actors))

(event EventSetSensedActorsKeys
  (params (Keys :type Array%20of%20Actor%20Object%20References))
  (Variables|Default|SetSensedActorsKeys Keys))

(event EventSetSensedActorsValues
  (params (Values :type Array%20of%20Floats%20%28single-precision%29))
  (Variables|Default|SetSensedActorsValues Values))

(event EventDetectedActor
  (params (Actor :type Actor%20Object%20Reference))
  (bind _returnvalue (Pawn|GetController))
  (bind _returnvalue_2 (AI|GetBlackboard _returnvalue))
  (Utilities|IsValid _returnvalue_2
    (:Is%20Valid
      (AI|Components|Blackboard|SetValueasBool _returnvalue_2 (Utilities|Name|MakeLiteralName "Alerted") true))))

(fn ConstructionScript
  (Transformation|SetWorldRotation (Math|Rotator|MakeRotator 0.0 (Variables|Default|GetBaseDirection) 0.0) false))

(fn GetActivelySensedActors
  (return (Variables|Default|GetActivelySensedActors)))

(fn GetSensedActorsKeys
  (return (Variables|Default|GetSensedActorsKeys)))

(fn GetSensedActorsValues
  (return (Variables|Default|GetSensedActorsValues)))

(fn UpdateStimuli
  (params (Actor :type Actor%20Object%20Reference) (StimulusAmount :type Float%20%28single-precision%29) (ReceiverLocation :type Vector :default "0, 0, 0") (StimulusLocation :type Vector :default "0, 0, 0") (SenseClass :type AI%20Sense%20Class%20Reference))
  (if (== SenseClass "/Script/AIModule.AISense_Sight")
    (bind _asthe_ultimate_heist_character (Utilities|Casting|CastToTheUltimateHeistCharacter Actor))
    (LocalVariables|SetValue (* (Math|Float|SelectFloat (- 1e+02 (Variables|/Script/TheUltimateHeist.TheUltimateHeistCharacter|GetConcealment _asthe_ultimate_heist_character)) 0.0 (Controller|LineOfSightTo (Pawn|GetController) Actor "0, 0, 0" false)) (Utilities|Time|GetWorldDeltaSeconds) (Variables|Default|GetDetectSpeed))))
  (return (LocalVariables|GetValue)))