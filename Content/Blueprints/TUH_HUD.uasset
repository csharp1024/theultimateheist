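; TUH_HUD is the stealth HUD, drawing a crosshair, a detection meter, per-AI awareness markers and debug text of sense levels.
; Tick finds the highest sense value any AI holds on the owning pawn and feeds it to a dynamic detection material.
; DrawHUD marks alerted AIs with red exclamations and sensing ones with blue question marks.
; DrawIndicator projects icons above actors, placing off-screen or behind-view ones around screen center with direction arrows.
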(event EventBeginPlay)

(event EventActorBeginOverlap
  (params (OtherActor :type Actor%20Object%20Reference)))

(event EventTick
  (params (DeltaSeconds :type Float%20%28single-precision%29))
  (bind _returnvalue (Class|HUD|GetOwningPawn))
  ;[1 1 1] Set max detection amount for indicator
  (Variables|Default|SetMaxDetection 0.0)
  (Utilities|IsValid _returnvalue
    (:Is%20Valid
      (bind _outactors (Actor|GetAllActorsOfClass "/Script/TheUltimateHeist.TUH_AICharacter"))
      (for _array_element _outactors
        (for (_array_element_2 _array_index) (Variables|/Script/TheUltimateHeist.TUH_AICharacter|GetSensedActorsKeys _array_element)
          (if (== _array_element_2 _returnvalue)
            (if (> (Utilities|Array|Get(acopy) (Variables|/Script/TheUltimateHeist.TUH_AICharacter|GetSensedActorsValues _array_element) _array_index) (Variables|Default|GetMaxDetection))
              (Variables|Default|SetMaxDetection (Utilities|Array|Get(acopy) (Variables|/Script/TheUltimateHeist.TUH_AICharacter|GetSensedActorsValues _array_element) _array_index))))))
      (Rendering|Material|SetScalarParameterValue (Variables|Default|GetDetectionMaterial) "DetectionAmount" (/ (Variables|Default|GetMaxDetection) 1e+02) :!class /Script/Engine.MaterialInstanceDynamic))))

(event EventDrawHUD
  (params (SizeX :type Integer) (SizeY :type Integer))
  (bind _returnvalue (Math|Float|MakeLiteralFloat 128.0))
  (bind _returnvalue_2 (/ _returnvalue 2.0))
  (Variables|Default|SetHalfScreenX (/ (Math|Conversions|ToFloat(Integer) SizeX) 2.0))
  (Variables|Default|SetHalfScreenY (/ (Math|Conversions|ToFloat(Integer) SizeY) 2.0))
  (Utilities|FlowControl|Sequence
    (:then_0
      ;[1 1 1] Draw Debug Info for AI Sense levels
      (bind _outactors (Actor|GetAllActorsOfClass "/Script/TheUltimateHeist.TUH_AICharacter"))
      (Variables|Default|SetX 0.0)
      (for _array_element _outactors
        (Variables|Default|SetY 0.0)
        (Utilities|FlowControl|Sequence
          (:then_0
            ;[1 1 1] Draw Actor Head Indicator
            (bind _asbp_tuh_aicharacter (Utilities|Casting|CastToBP_TUH_AICharacter _array_element))
            (if (Variables|/Game/Blueprints/AI/BP_TUH_AICharacter.BP_TUH_AICharacter_C|GetAlerted _asbp_tuh_aicharacter)
              (if false
                (CallFunction|DrawIndicator _asbp_tuh_aicharacter "(R=1.000000,G=0.000000,B=0.109804,A=1.000000)" "/Game/Textures/phone.phone")
                (else
                  (CallFunction|DrawIndicator _asbp_tuh_aicharacter "(R=1.000000,G=0.000000,B=0.109804,A=1.000000)" "/Game/Textures/exclamation.exclamation")))
              (elif (> (Utilities|Array|Length (Variables|/Script/TheUltimateHeist.TUH_AICharacter|GetSensedActorsKeys _asbp_tuh_aicharacter)) 0)
                (CallFunction|DrawIndicator _asbp_tuh_aicharacter "(R=0.000000,G=0.588293,B=1.000000,A=1.000000)" "/Game/Textures/question.question"))))
          (:then_1
            (Variables|Default|SetX (+ (Variables|Default|GetX) 2e+02))
            (HUD|DrawText (Utilities|GetDisplayName _array_element) "(R=0,G=0,B=0,A=1)" (Variables|Default|GetX) (Variables|Default|GetY) 0 1.1 false)
            (Variables|Default|SetY (+ (Variables|Default|GetY) 2e+01))
            (for (_array_element_2 _array_index) (Variables|/Script/TheUltimateHeist.TUH_AICharacter|GetSensedActorsKeys _array_element)
              (HUD|DrawText (Utilities|GetDisplayName _array_element_2) "(R=0.360142,G=0.368871,B=0.820000,A=1.000000)" (Variables|Default|GetX) (Variables|Default|GetY) "/Engine/EngineFonts/Roboto.Roboto" 1.0 false)
              (HUD|DrawText (Utilities|String|ToString(Text) (Utilities|Text|ToText(Float) (Utilities|Array|Get(acopy) (Variables|/Script/TheUltimateHeist.TUH_AICharacter|GetSensedActorsValues _array_element) _array_index) "HalfToEven")) "(R=0.965000,G=0.008871,B=0.045741,A=1.000000)" (+ (Variables|Default|GetX) (.OutWidth (Class|HUD|GetTextSize (Utilities|GetDisplayName _array_element_2) "/Engine/EngineFonts/Roboto.Roboto" 1.0))) (Variables|Default|GetY) "/Engine/EngineFonts/Roboto.Roboto" 1.0 false)
              (Variables|Default|SetY (+ (Variables|Default|GetY) 14.0)))))))
    (:then_1
      ;[1 1 1] Draw Crosshair
      (Canvas|DrawTexture (Variables|Default|GetCrosshair) (- (Variables|Default|GetHalfScreenX) 8.0) (- (Variables|Default|GetHalfScreenY) 8.0) 16.0 16.0 0.0 0.0 1.0 1.0 "(R=1.000000,G=1.000000,B=1.000000,A=1.000000)"))
    (:then_2
      ;[1 1 1] Draw Detection Indicator
      (Canvas|DrawMaterial (Variables|Default|GetDetectionMaterial) (- (Variables|Default|GetHalfScreenX) _returnvalue_2) (- (Variables|Default|GetHalfScreenY) _returnvalue_2) _returnvalue _returnvalue 0.0 0.0 1.0 1.0 1.0 false 9e+01 "(X=0.500000,Y=0.500000)"))))

(fn ConstructionScript
  (bind _returnvalue (Rendering|Material|CreateDynamicMaterialInstance "/Game/Materials/Detection.Detection" :!class /Script/Engine.KismetMaterialLibrary))
  (Variables|Default|SetDetectionMaterial _returnvalue)
  (bind _returnvalue_2 (Rendering|Material|CreateDynamicMaterialInstance "/Game/Materials/Interaction.Interaction" :!class /Script/Engine.KismetMaterialLibrary))
  (Variables|Default|SetInteractionMaterial _returnvalue_2))

(fn DrawIndicator
  (params (Actor :type Actor%20Object%20Reference) (Color :type Linear%20Color%20Structure) (Icon :type Texture%202D%20Object%20Reference))
  (bind _returnvalue (Class|HUD|GetOwningPawn))
  (bind _returnvalue_2 (Transformation|GetActorLocation Actor))
  (bind _returnvalue_3 (Math|Float|MakeLiteralFloat 32.0))
  (bind _returnvalue_4 (Math|Float|MakeLiteralFloat 32.0))
  (bind _returnvalue_5 (Math|Float|MakeLiteralFloat 128.0))
  (bind _halfscreenx (Variables|Default|GetHalfScreenX))
  (bind _halfscreeny (Variables|Default|GetHalfScreenY))
  (bind _halfscreenx_2 (Variables|Default|GetHalfScreenX))
  (bind _halfscreeny_2 (Variables|Default|GetHalfScreenY))
  (bind _halfscreenx_3 (Variables|Default|GetHalfScreenX))
  (bind _halfscreeny_3 (Variables|Default|GetHalfScreenY))
  (bind _halfscreenx_4 (Variables|Default|GetHalfScreenX))
  (bind _halfscreeny_4 (Variables|Default|GetHalfScreenY))
  (bind _returnvalue_6 (Transformation|GetActorLocation _returnvalue))
  (bind _returnvalue_7 (/ _returnvalue_3 2.0))
  (bind _returnvalue_8 (Transformation|GetActorRotation _returnvalue))
  (bind _returnvalue_9 (/ _returnvalue_4 2.0))
  (bind _returnvalue_10 (+ _returnvalue_2 "0, 0,100.000000"))
  (bind _returnvalue_11 (Math|Float|Min(Float) _halfscreenx_3 _halfscreeny_3))
  (bind _returnvalue_12 (Class|HUD|Project _returnvalue_10))
  (bind _returnvalue_13 (- _returnvalue_2 _returnvalue_6))
  (bind _returnvalue_14 (- (.x _returnvalue_12) _halfscreenx_4))
  (bind _returnvalue_15 (- (.y _returnvalue_12) _halfscreeny_4))
  (bind _returnvalue_16 (Math|Vector|UnrotateVector _returnvalue_13 _returnvalue_8))
  (bind _returnvalue_17 (== (.z _returnvalue_12) 0.0))
  (bind _returnvalue_18 (Math|Float|Absolute(Float) _returnvalue_14))
  (bind _returnvalue_19 (Math|Float|Absolute(Float) _returnvalue_15))
  (bind _returnvalue_20 (Math|Vector|RotateVectorAroundAxis _returnvalue_16 -9e+01 "0, 0,1.000000"))
  (bind _returnvalue_21 (Math|Vector|MakeVector _returnvalue_14 _returnvalue_15 0.0))
  (bind _returnvalue_22 (Math|Vector|Normalize _returnvalue_20))
  (bind _returnvalue_23 (- _returnvalue_18 _halfscreenx_2))
  (bind _returnvalue_24 (- _returnvalue_19 _halfscreeny_2))
  (bind _returnvalue_25 (Math|Vector|Normalize _returnvalue_21))
  (bind _returnvalue_26 (* _returnvalue_22 _returnvalue_5))
  (bind _returnvalue_27 (Math|Float|Max(Float) _returnvalue_23 _returnvalue_24))
  (bind _returnvalue_28 (- _returnvalue_11 _returnvalue_27))
  (bind _returnvalue_29 (Math|Float|Clamp(Float) _returnvalue_28 0.0 _returnvalue_11))
  (bind _returnvalue_30 (+ _returnvalue_5 _returnvalue_29))
  (bind _returnvalue_31 (Math|Float|SelectFloat _returnvalue_5 _returnvalue_30 _returnvalue_17))
  (bind _returnvalue_32 (* _returnvalue_25 _returnvalue_31))
  (bind _returnvalue_33 (Math|Vector|SelectVector _returnvalue_26 _returnvalue_32 _returnvalue_17))
  (bind _returnvalue_34 (Math|Vector|Normalize _returnvalue_33))
  (bind _returnvalue_35 (+ _returnvalue_33 (Math|Vector|MakeVector _halfscreenx _halfscreeny 0.0)))
  (bind _returnvalue_36 (* _returnvalue_34 _returnvalue_4))
  (bind _returnvalue_37 (+ _returnvalue_35 _returnvalue_36))
  (Utilities|IsValid _returnvalue
    (:Is%20Valid
      (LocalVariables|SetScreenSpace (Math|Vector|MakeVector (.x _returnvalue_12) (.y _returnvalue_12) (.z _returnvalue_12)))
      (if (Math|Boolean|ORBoolean (> _returnvalue_18 _halfscreenx_4) (> _returnvalue_19 _halfscreeny_4) _returnvalue_17)
        (LocalVariables|SetScreenSpace _returnvalue_35)
        (Canvas|DrawTexture "/Game/Textures/arrow.arrow" (- (.x _returnvalue_37) _returnvalue_7) (- (.y _returnvalue_37) _returnvalue_7) _returnvalue_3 _returnvalue_3 0.0 0.0 1.0 1.0 Color "BLEND_Translucent" 1.0 false (+ (.yaw (Math|Conversions|RotationFromXVector _returnvalue_33)) 9e+01) "(X=0.500000,Y=0.500000)"))
      (Canvas|DrawTexture Icon (- (.x (LocalVariables|GetScreenSpace)) _returnvalue_9) (- (.y (LocalVariables|GetScreenSpace)) _returnvalue_9) _returnvalue_4 _returnvalue_4 0.0 0.0 1.0 1.0 Color))))